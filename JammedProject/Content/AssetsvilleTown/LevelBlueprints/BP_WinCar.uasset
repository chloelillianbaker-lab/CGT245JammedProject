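; BP_WinCar is a pushable car block that triggers the win condition when its Box overlaps any actor other than the player.
; On a player hit, a forward line trace confirms the player faces the car along the Y axis.
; The MoveBlock timeline then slides it by TravelDistance in that direction, without sweep.
; Winning shows the Win widget, unpauses the game and destroys the player character.
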(event OnComponentBeginOverlap(Box)
  (params (OverlappedComponent :type Primitive%20Component%20Object%20Reference) (OtherActor :type Actor%20Object%20Reference) (OtherComp :type Primitive%20Component%20Object%20Reference) (OtherBodyIndex :type Integer) (bFromSweep :type Boolean) (SweepResult :type Hit%20Result%20Structure%20%28by%20ref%29))
  (if (!= (Game|GetPlayerCharacter 0) OtherActor)
    (CallFunction|Win)))

(event Custom|Push
  (Variables|Default|SetcurrentLocation (Transformation|GetActorLocation))
  (bind _position (Timeline|MoveBlock PlayFromStart)
    (:Update
      (Transformation|SetActorRelativeLocation (+ (Variables|Default|GetcurrentLocation) (* _position (Variables|Default|GetPushableDirection) (Variables|Default|GetTravelDistance)))))))

(event Custom|Win
  (bind _returnvalue (UserInterface|CreateWidget "/Game/AssetsvilleTown/LevelBlueprints/win.win_C" (Game|GetPlayerController 0)))
  (UserInterface|Viewport|AddtoViewport _returnvalue 0)
  (Game|SetGamePaused false)
  (Actor|DestroyActor (Game|GetPlayerCharacter 0)))

(event Collision|EventHit
  (params (MyComp :type Primitive%20Component%20Object%20Reference) (Other :type Actor%20Object%20Reference) (OtherComp :type Primitive%20Component%20Object%20Reference) (bSelfMoved :type Boolean) (HitLocation :type Vector :default "0, 0, 0") (HitNormal :type Vector :default "0, 0, 0") (NormalImpulse :type Vector :default "0, 0, 0") (Hit :type Hit%20Result%20Structure%20%28by%20ref%29))
  (if (== (Game|GetPlayerCharacter 0) Other)
    (Variables|Default|SetPushableDirection (Math|Vector|MakeVector 0.0 (Math|Conversions|ToFloat(Integer) (Math|Float|Round (.Y (Math|Vector|BreakVector (Transformation|GetActorForwardVector Other))))) 0.0))
    (bind _canpush (CallFunction|CanPush))
    (if _canpush
      (CallFunction|Push))))

(fn ConstructionScript)

(fn CanPush
  (bind _returnvalue (Game|GetPlayerCharacter 0))
  (bind _returnvalue_2 (Transformation|GetActorLocation _returnvalue))
  (bind (_outhit _returnvalue_3) (Collision|LineTraceByChannel _returnvalue_2 (+ _returnvalue_2 (* (Transformation|GetActorForwardVector _returnvalue) 1e+02)) "TraceTypeQuery1" false (Utilities|Array|MakeArray _returnvalue) "None" false))
  (if _returnvalue_3
    (if (== (.HitActor (Collision|BreakHitResult _outhit)) self)
      (if (== (Math|Float|Round (.X (Math|Vector|BreakVector (Transformation|GetActorForwardVector (Game|GetPlayerCharacter 0))))) 0)
        (return true)
        (else
          (return false)))
      (else
        (return false)))
    (else
      (return false))))