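; BP_Car7 is a car the player shoves along the world X axis by walking into it.
; On a player hit, CanPush uses a forward line trace and the player's facing, then a Timeline slides the car from its current location by TravelDistance.
; Each update, IsBlocked picks the Front or Back overlap component by travel direction and skips the move when it has more than one overlapping actor.
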(event Custom|Push
  (Variables|Default|SetcurrentLocation (Transformation|GetActorLocation))
  (bind _position (Timeline|Timeline PlayFromStart)
    (:Update
      (bind _blocked (CallFunction|IsBlocked (* _position (Variables|Default|GetPushableDirection) (Variables|Default|GetTravelDistance))))
      (if (not _blocked)
        (Transformation|SetActorRelativeLocation (+ (Variables|Default|GetcurrentLocation) (* _position (Variables|Default|GetPushableDirection) (Variables|Default|GetTravelDistance))))))))

(event Collision|EventHit
  (params (MyComp :type Primitive%20Component%20Object%20Reference) (Other :type Actor%20Object%20Reference) (OtherComp :type Primitive%20Component%20Object%20Reference) (bSelfMoved :type Boolean) (HitLocation :type Vector :default "0, 0, 0") (HitNormal :type Vector :default "0, 0, 0") (NormalImpulse :type Vector :default "0, 0, 0") (Hit :type Hit%20Result%20Structure%20%28by%20ref%29))
  (if (== (Game|GetPlayerCharacter 0) Other)
    (Variables|Default|SetPushableDirection (Math|Vector|MakeVector (Math|Conversions|ToFloat(Integer) (Math|Float|Round (.X (Math|Vector|BreakVector (Transformation|GetActorForwardVector Other))))) 0.0 0.0))
    (bind _canpush (CallFunction|CanPush))
    (if _canpush
      (CallFunction|Push))))

(fn ConstructionScript)

(fn CanPush
  (bind _returnvalue (Game|GetPlayerCharacter 0))
  (bind _returnvalue_2 (Transformation|GetActorLocation _returnvalue))
  (bind (_outhit _returnvalue_3) (Collision|LineTraceByChannel _returnvalue_2 (+ _returnvalue_2 (* (Transformation|GetActorForwardVector _returnvalue) 1e+02)) "TraceTypeQuery1" false (Utilities|Array|MakeArray _returnvalue) "None" false))
  (if _returnvalue_3
    (if (== (.HitActor (Collision|BreakHitResult _outhit)) self)
      (if (== (Math|Float|Round (.Y (Math|Vector|BreakVector (Transformation|GetActorForwardVector (Game|GetPlayerCharacter 0))))) 0)
        (return true)
        (else
          (return false)))
      (else
        (return false)))
    (else
      (return true))))

(fn IsBlocked
  (params (direction :type Vector))
  (Math|Float|CompareFloat (Math|Vector|DotProduct (Transformation|GetActorForwardVector) direction) 0.0
    (:>
      (Math|Integer|CompareInt (Utilities|Array|Length (Collision|GetOverlappingActors (Variables|Default|GetFront) 0 :!class /Script/Engine.PrimitiveComponent)) 1
        (:>
          (return true))
        (:==
          _)
        (:<
          _))
      (return false))
    (:<
      (Math|Integer|CompareInt (Utilities|Array|Length (Collision|GetOverlappingActors (Variables|Default|GetBack) 0 :!class /Script/Engine.PrimitiveComponent)) 1
        (:>
          (return true))
        (:==
          _)
        (:<
          _))
      (return false))))